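; BP_Enemy_Snail is a snail enemy that crawls forward, turns at walls and ledges, and damages players it touches.
; Its MoveForward event adds forward movement input, sets the attack flag and damage, and reveals the HitBox.
; WallDetector begin-overlap and LedgeDetector end-overlap both flip the actor 180 degrees through TurnChar.
; HitBox overlaps run HitCheck, which applies BaseDamage to every overlapping BP_Player.
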(event OnComponentBeginOverlap(WallDetector)
  (params (OverlappedComponent :type Primitive%20Component%20Object%20Reference) (OtherActor :type Actor%20Object%20Reference) (OtherComp :type Primitive%20Component%20Object%20Reference) (OtherBodyIndex :type Integer) (bFromSweep :type Boolean) (SweepResult :type Hit%20Result%20Structure%20%28by%20ref%29))
  (CallFunction|TurnChar))

(event OnComponentEndOverlap(LedgeDetector)
  (params (OverlappedComponent :type Primitive%20Component%20Object%20Reference) (OtherActor :type Actor%20Object%20Reference) (OtherComp :type Primitive%20Component%20Object%20Reference) (OtherBodyIndex :type Integer))
  (CallFunction|TurnChar))

(event OnComponentBeginOverlap(HitBox)
  (params (OverlappedComponent :type Primitive%20Component%20Object%20Reference) (OtherActor :type Actor%20Object%20Reference) (OtherComp :type Primitive%20Component%20Object%20Reference) (OtherBodyIndex :type Integer) (bFromSweep :type Boolean) (SweepResult :type Hit%20Result%20Structure%20%28by%20ref%29))
  (CallFunction|HitCheck))

(event Custom|MoveForward
  (Pawn|Input|AddMovementInput (Transformation|GetActorForwardVector) 1.0 false)
  (Variables|Default|SetAttack true)
  (Variables|Default|SetBase%20Damage 25.0)
  (Development|SetHiddeninGame (Variables|Default|GetHitBox) false false))

(event Collision|EventActorBeginOverlap
  (params (OtherActor :type Actor%20Object%20Reference)))

(fn ConstructionScript)

(fn TurnChar
  (Transformation|SetActorRotation (Math|Rotator|CombineRotators (Transformation|GetActorRotation) "0.000000,180.000000,0.000000")))

(fn HitCheck
  (for _array_element (Collision|GetOverlappingActors (Variables|Default|GetHitBox) "/Game/Blueprints/BP_Player.BP_Player_C" :!class /Script/Engine.PrimitiveComponent)
    (if (!= _array_element self)
      (Game|Damage|ApplyDamage _array_element (Variables|Default|GetBase%20Damage) 0 0))))